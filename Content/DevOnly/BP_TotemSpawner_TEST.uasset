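; Dev-only test spawner that scatters totem actors through a box volume when play begins.
; A BeginPlay loop driven by TotemCount spawns TotemClass at random points within the Box bounds, each with a random yaw.
; Each totem receives a random difficulty from the first three EOryxTotemDifficulty values.
; Spawns adjust for collision where possible but always go through.
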(event EventBeginPlay
  (bind _box (Variables|Default|GetBox))
  (for _index (range 0 (Variables|Default|GetTotemCount))
    (Game|SpawnActorfromClass (Variables|Default|GetTotemClass) (Math|Transform|MakeTransform (Math|Random|RandomPointinBoundingBox (Transformation|GetWorldLocation _box) (Components|Box|GetScaledBoxExtent _box)) (Math|Rotator|MakeRotator 0.0 0.0 (Math|Random|RandomFloatinRange 0.0 3.6e+02)) "1.000000,1.000000,1.000000") "AdjustIfPossibleButAlwaysSpawn" "MultiplyWithRoot" 0 (Utilities|Enum|ByteToEnumEOryxTotemDifficulty (Math|Conversions|ToByte(Integer) (Math|Random|RandomIntegerinRange 0 2))) 0)))

(fn ConstructionScript)