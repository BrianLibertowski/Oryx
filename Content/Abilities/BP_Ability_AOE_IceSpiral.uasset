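; BP_Ability_AOE_IceSpiral is an area-of-effect ability that damages pawns around its owner.
; On Activate, it spawns the VFX system at the owner's location and runs a single sphere overlap of the configured Radius there, ignoring the owner.
; Each overlapped actor with a valid OryxHealthComponent receives Damage through that component's ApplyDamage.
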(event EventActivate
  (params (Owner :type Actor%20Object%20Reference))
  (bind _returnvalue (Transformation|GetActorLocation Owner))
  (Niagara|SpawnSystematLocation self (Variables|Default|GetVFX) _returnvalue)
  (bind _outactors (Collision|SphereOverlapActors self _returnvalue (Variables|Default|GetRadius) (Utilities|Array|MakeArray "ObjectTypeQuery3") 0 (Utilities|Array|MakeArray Owner)))
  (for _array_element _outactors
    (Utilities|IsValid (Actor|GetComponentbyClass _array_element "/Script/Oryx.OryxHealthComponent")
      (:Is%20Valid
        (Class|OryxHealthComponent|ApplyDamage (Actor|GetComponentbyClass _array_element "/Script/Oryx.OryxHealthComponent") (Variables|Default|GetDamage))))))