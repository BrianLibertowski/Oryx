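; Fire Arrows area-of-effect ability that burns and damages pawns around its owner.
; On activation it tries to spend mana from the owning BP_OryxCharacter, then spawns a VFX system at the owner's location.
; A sphere overlap gathers nearby pawns except the owner.
; Each one with an OryxHealthComponent receives a status effect through OryxStatusEffectsComponent, which is not validity-checked, then a Fire damage event.
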(event EventActivate
  (params (Owner :type Actor%20Object%20Reference))
  (bind _returnvalue (Transformation|GetActorLocation Owner))
  ;[0.15 0.15 0.15 0.5] FireArrows AOE Ability
  ;;[0.15 0.15 0.15 0.5] Consume Mana On Ability Usage
  (bind _asbp_oryx_character (Utilities|Casting|CastToBP_OryxCharacter Owner))
  (bind _returnvalue_2 (Class|OryxCharacter|TryConsumeMana _asbp_oryx_character 25.0))
  (if _returnvalue_2
    ;;[0.15 0.15 0.15 0.5] Spawn VFX
    (Niagara|SpawnSystematLocation self (Variables|Default|GetVFX) _returnvalue)
    ;;[0.15 0.15 0.15 0.5] Area/Radius
    (bind _outactors (Collision|SphereOverlapActors self _returnvalue (Variables|Default|GetRadius) (Utilities|Array|MakeArray "ObjectTypeQuery3") 0 (Utilities|Array|MakeArray Owner)))
    (for _array_element _outactors
      (Utilities|IsValid (Actor|GetComponentbyClass _array_element "/Script/Oryx.OryxHealthComponent")
        (:Is%20Valid
          (Class|OryxStatusEffectsComponent|ApplyEffect (Actor|GetComponentbyClass _array_element "/Script/Oryx.OryxStatusEffectsComponent") (Utilities|Struct|MakeOryxStatusEffectSpec "Burn" 4.0 0.5 0.4 Owner))
          (Class|OryxHealthComponent|ApplyDamageEvent (Actor|GetComponentbyClass _array_element "/Script/Oryx.OryxHealthComponent") (Utilities|Struct|MakeOryxDamageEvent (Variables|Default|GetDamage) "Fire" Owner Owner)))))))