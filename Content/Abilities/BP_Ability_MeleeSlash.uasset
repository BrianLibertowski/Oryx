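; Melee slash ability that damages pawns in front of its owner on activation, as a placeholder until a real swing exists.
; Activate runs a debug-drawn multi-sphere trace from the owner along its forward vector, sized by Range and Radius.
; Each hit actor is processed once via DamagedActors, and those with an OryxHealthComponent receive an Oryx damage event crediting the owner as instigator and causer.
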(event EventActivate
  (params (Owner :type Actor%20Object%20Reference))
  (bind _returnvalue (Transformation|GetActorLocation Owner))
  ;[0 0.75 1] On Melee hit/swing Apply Damage - PlaceHolder requires actuall swing
  (Variables|Default|SetDamagedActors (Utilities|Array|MakeArray 0))
  (bind _outhits (Collision|MultiSphereTraceForObjects Owner _returnvalue (+ _returnvalue (* (Transformation|GetActorForwardVector Owner) (Variables|Default|GetRange))) (Variables|Default|GetRadius) (Utilities|Array|MakeArray "ObjectTypeQuery3") false (Utilities|Array|MakeArray Owner) "ForDuration"))
  (for _array_element _outhits
    (if (not (Utilities|Array|ContainsItem (Variables|Default|GetDamagedActors) (.HitActor (Collision|BreakHitResult _array_element))))
      (Utilities|Array|Add (Variables|Default|GetDamagedActors) (.HitActor (Collision|BreakHitResult _array_element)))
      (if (!= (.HitActor (Collision|BreakHitResult _array_element)) Owner)
        (Utilities|IsValid (Actor|GetComponentbyClass (.HitActor (Collision|BreakHitResult _array_element)) "/Script/Oryx.OryxHealthComponent")
          (:Is%20Valid
            (Class|OryxHealthComponent|ApplyDamageEvent (Actor|GetComponentbyClass (.HitActor (Collision|BreakHitResult _array_element)) "/Script/Oryx.OryxHealthComponent") (Utilities|Struct|MakeOryxDamageEvent (Variables|Default|GetDamage) "Physical" Owner Owner))))))))