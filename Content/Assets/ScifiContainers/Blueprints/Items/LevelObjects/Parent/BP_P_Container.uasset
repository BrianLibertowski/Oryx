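; Parent Blueprint for sci-fi container level props, setting up their doors and appearance at construction time.
; The construction script runs InitDoors, then EditAppearance on the Base and each static mesh child of Doors.
; Appearance is written as default custom primitive data: a constant flag, Color, and damage/dirt amount.
; Damage/dirt uses DamageDirtAmount or, with FullyRandom, a separate seeded-stream draw per mesh.
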(event EventBeginPlay)

(event EventTick
  (params (DeltaSeconds :type Float%20%28single-precision%29))
  (|CallParentFunction DeltaSeconds) ; This node is disabled and will not be called.\nDrag off pins to build functionality.
)

(fn ConstructionScript
  (|CallParentFunction)
  (CallFunction|InitDoors)
  (CallFunction|EditAppearance))

(fn EditAppearance
  (bind _damage_dirtamount (Variables|Control|GetDamage/DirtAmount))
  (bind _base (Variables|Default|GetBase))
  (bind _color (Variables|Control|GetColor))
  (bind _color_2 (Variables|Control|GetColor))
  (bind _fullyrandom (Variables|Default|GetFullyRandom))
  (bind _randomseedstruct (Variables|Default|GetRandomSeedStruct))
  (bind _returnvalue (Math|Random|RandomFloatinRangefromStream _randomseedstruct 1.0 2.0))
  (bind _returnvalue_2 (select _fullyrandom _returnvalue _damage_dirtamount))
  (Rendering|Material|SetDefaultCustomPrimitiveDataFloat (Variables|Default|GetBase) 0 1.0)
  (Rendering|Material|SetDefaultCustomPrimitiveDataVector4 _base 2 (Math|Vector4|MakeVector4 (.r _color_2) (.g _color_2) (.b _color_2) 0.0))
  (Rendering|Material|SetDefaultCustomPrimitiveDataFloat _base 1 _returnvalue_2)
  (for _array_element (Components|GetChildrenComponents (Variables|Default|GetDoors) false)
    (bind _asstatic_mesh_component (Utilities|Casting|CastToStaticMeshComponent _array_element))
    (Rendering|Material|SetDefaultCustomPrimitiveDataFloat _asstatic_mesh_component 0 1.0)
    (Rendering|Material|SetDefaultCustomPrimitiveDataVector4 _asstatic_mesh_component 2 (Math|Vector4|MakeVector4 (.r _color) (.g _color) (.b _color) 0.0))
    (Rendering|Material|SetDefaultCustomPrimitiveDataFloat _asstatic_mesh_component 1 _returnvalue_2)))