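; InspectPawn is an example player pawn with a cine camera that adds head bob and automatic depth-of-field focus.
; On BeginPlay it starts the BP_HeadBob camera shake on the first player controller.
; Every Tick it line-traces forward from the camera on the Visibility channel and uses the distance to the hit location as focal distance.
; It then rebuilds the camera's post-process settings with that focus and fixed aperture and blur values.
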(event EventBeginPlay
  (Game|Feedback|ClientStartCameraShake (Game|GetPlayerController 0) "/Game/Assets/ScifiContainers/ExamplePlayer/Blueprints/BP_HeadBob.BP_HeadBob_C" 5e+01 "World" "0, 0, 0"))

(event Collision|EventActorBeginOverlap
  (params (OtherActor :type Actor%20Object%20Reference)))

(event EventTick
  (params (DeltaSeconds :type Float%20%28single-precision%29))
  (bind _cinecamera (Variables|Default|GetCineCamera))
  (bind _returnvalue (Transformation|GetWorldLocation _cinecamera))
  (bind _outhit (Collision|LineTraceByChannel _returnvalue (+ _returnvalue (* (Math|Vector|GetForwardVector _cinecamera) (Variables|Default|GetAutoFocusTraceDistance))) "TraceTypeQuery1" true (Utilities|Array|MakeArray self) "None"))
  (Variables|Default|SetFocusLocation (Math|Vector|VectorLength (- (.Location (Collision|BreakHitResult _outhit)) (Transformation|GetWorldLocation (Variables|Default|GetCineCamera)))))
  (Variables|/Script/Engine.CameraComponent|SetPostProcessSettings (Variables|Default|GetCineCamera) (Utilities|Struct|MakePostProcessSettings 0.3 11.0 2.0 (Variables|Default|GetFocusLocation) 1.0 1e+01)))

(fn ConstructionScript)