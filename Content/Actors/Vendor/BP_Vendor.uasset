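; BP_Vendor is an interactable vendor actor that opens a shop screen for the interacting player.
; On Interact it prints a debug message, then creates VendorWidgetClass for the interactor's player controller, provided the class is valid.
; The WBP_VendorScreen is initialized with this vendor and added to the viewport.
; Input then switches to Game and UI with the screen focused and the mouse cursor shown.
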(event EventInteract
  (params (Interactor :type Oryx%20Character%20Object%20Reference))
  (Development|PrintString "Vendor open")
  (if (Utilities|IsValidClass (Variables|Default|GetVendorWidgetClass))
    (bind _asplayer_controller (Utilities|Casting|CastToPlayerController (Pawn|GetController Interactor)))
    (bind _returnvalue (UserInterface|CreateWidget (Variables|Default|GetVendorWidgetClass) _asplayer_controller))
    (bind _aswbp_vendor_screen (Utilities|Casting|CastToWBP_VendorScreen _returnvalue))
    (Default|InitforVendor _aswbp_vendor_screen self)
    (UserInterface|Viewport|AddtoViewport _aswbp_vendor_screen 0)
    (Input|SetInputModeGameandUI _asplayer_controller _aswbp_vendor_screen "DoNotLock" true false)
    (Variables|/Script/Engine.PlayerController|SetbShowMouseCursor _asplayer_controller true)))

(fn ConstructionScript)