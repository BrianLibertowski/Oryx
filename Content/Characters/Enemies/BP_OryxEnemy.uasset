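; BP_OryxEnemy is an enemy Blueprint that shows floating damage numbers when it takes damage.
; On BeginPlay it binds a handler to its HealthComponent's damage-received event.
; If Oryx settings enable damage numbers, the handler spawns a BP_FloatingDamageActor above the enemy, passing final damage, damage type and crit flag.
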(event Custom|HandleDamageReceived
  (params (Event :type Oryx%20Damage%20Event%20Structure) (FinalDamage :type Float%20%28single-precision%29) (bWasCrit :type Boolean))
  ;[0.15 0.15 0.15 0.5] On Enemy Damage Received Show Corresponding Damage Type - Floating Numbers
  (if (Class|OryxGameUserSettings|GetShowFloatingDamageNumbers (Class|OryxGameUserSettings|GetOryxSettings))
    (Game|SpawnActorfromClass "/Game/UI/HUD/BP_FloatingDamageActor.BP_FloatingDamageActor_C" (Math|Transform|MakeTransform (+ (Transformation|GetActorLocation) "0.000000,0.000000,120.000000")) "AlwaysSpawn" "MultiplyWithRoot" 0 FinalDamage (.DamageType (Utilities|Struct|BreakOryxDamageEvent Event)) bWasCrit 0)))

(event EventBeginPlay
  ;[0.15 0.15 0.15 0.5] On Enemy Damage Received Show Corresponding Damage Type - Floating Numbers
  (EventDispatchers|BindEventtoOnDamageReceived (Variables|Default|GetHealthComponent) (delegate Custom|HandleDamageReceived)))

(fn ConstructionScript)