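; Boss enemy MegaGrizzleBark for the first stage, adding a telegraphed heavy ground slam on top of its parent enemy behavior.
; A looping timer periodically starts a telegraph when the forced target is valid and within range, unless one is already running.
; The telegraph event halts movement for the windup, then slams and restores walk speed.
; The slam sphere-overlaps nearby pawns and deals amplified physical damage to Oryx characters.
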(event Custom|HandleTelegraph
  (params (WindupSeconds :type Float%20%28single-precision%29))
  (bind _charactermovement (Variables|Character|GetCharacterMovement))
  (Variables|/Script/Engine.CharacterMovementComponent|SetMaxWalkSpeed _charactermovement 0.0)
  (Utilities|FlowControl|Delay WindupSeconds)
  (CallFunction|DoHeavySlam)
  (Variables|/Script/Engine.CharacterMovementComponent|SetMaxWalkSpeed _charactermovement 3e+02))

(event Custom|TryTelegraph
  (bind _returnvalue (Class|OryxEnemy|GetForcedTarget))
  (if (not (Class|OryxBoss|IsTelegraphingAttack))
    (Utilities|IsValid _returnvalue
      (:Is%20Valid
        (if (< (Transformation|GetDistanceTo _returnvalue) 6e+02)
          (Class|OryxBoss|TelegraphAttack 1.5))))))

(event Custom|DoHeavySlam
  (bind _outactors (Collision|SphereOverlapActors (Transformation|GetActorLocation) 5.5e+02 (Utilities|Array|MakeArray "ObjectTypeQuery3") 0 (Utilities|Array|MakeArray self)))
  (for _array_element _outactors
    (bind _asoryx_character (Utilities|Casting|CastToOryxCharacter _array_element))
    (Class|OryxHealthComponent|ApplyDamageEvent (Variables|/Script/Oryx.OryxCharacter|GetHealthComponent _asoryx_character) (Utilities|Struct|MakeOryxDamageEvent (* (Class|OryxEnemy|GetAttackDamage) 2.5) "Physical" self))))

(event EventBeginPlay
  (|CallParentFunction)
  (EventDispatchers|AssignOnTelegraphAttack (delegate Custom|HandleTelegraph))
  (Utilities|Time|SetTimerbyEvent (delegate Custom|TryTelegraph) 8.0 true))

(fn ConstructionScript)