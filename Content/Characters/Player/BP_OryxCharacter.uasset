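; BP_OryxCharacter is the player character, wiring input to abilities and adding damage feedback and a stats screen.
; Enhanced Input actions for fire and five AOE spells activate fixed slot indices on the AbilityComponent.
; HealthComponent damage events spawn floating damage-number actors above the character when enabled in Oryx settings.
; BeginPlay sets game-only input for the locally controlled player, and a toggle event creates or removes the stats widget.
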(event Custom|HandleDamageReceived
  (params (Event :type Oryx%20Damage%20Event%20Structure) (FinalDamage :type Float%20%28single-precision%29) (bWasCrit :type Boolean))
  (if (Class|OryxGameUserSettings|GetShowFloatingDamageNumbers (Class|OryxGameUserSettings|GetOryxSettings))
    (Game|SpawnActorfromClass "/Game/UI/HUD/BP_FloatingDamageActor.BP_FloatingDamageActor_C" (Math|Transform|MakeTransform (+ (Transformation|GetActorLocation) "0.000000,0.000000,120.000000")) "AlwaysSpawn" "MultiplyWithRoot" 0 FinalDamage (.DamageType (Utilities|Struct|BreakOryxDamageEvent Event)) bWasCrit 0)))

(event Input|EnhancedActionEvents|EnhancedInputActionIA_Fire
  (params (ActionValue :type Boolean) (ElapsedSeconds :type Float%20%28double-precision%29) (TriggeredSeconds :type Float%20%28double-precision%29) (InputAction :type Input%20Action%20Object%20Reference :default "/Game/Input/Actions/IA_Fire.IA_Fire"))
  ;[0.15 0.15 0.15 0.5] Abilities
  (:Started
    (Class|OryxAbilityComponent|TryActivateAbility (Variables|Default|GetAbilityComponent))))

(event Input|EnhancedActionEvents|EnhancedInputActionIA_Ability_AOE_Blaze
  (params (ActionValue :type Boolean) (ElapsedSeconds :type Float%20%28double-precision%29) (TriggeredSeconds :type Float%20%28double-precision%29) (InputAction :type Input%20Action%20Object%20Reference :default "/Game/Input/Actions/IA_Ability_AOE_Blaze.IA_Ability_AOE_Blaze"))
  ;[0.15 0.15 0.15 0.5] Abilities
  (:Started
    (Class|OryxAbilityComponent|TryActivateAbility (Variables|Default|GetAbilityComponent) 2)))

(event Input|EnhancedActionEvents|EnhancedInputActionIA_Ability_AOE_Blizzard
  (params (ActionValue :type Boolean) (ElapsedSeconds :type Float%20%28double-precision%29) (TriggeredSeconds :type Float%20%28double-precision%29) (InputAction :type Input%20Action%20Object%20Reference :default "/Game/Input/Actions/IA_Ability_AOE_Blizzard.IA_Ability_AOE_Blizzard"))
  ;[0.15 0.15 0.15 0.5] Abilities
  (:Started
    (Class|OryxAbilityComponent|TryActivateAbility (Variables|Default|GetAbilityComponent) 3)))

(event Input|EnhancedActionEvents|EnhancedInputActionIA_Ability_AOE_FireArrows
  (params (ActionValue :type Boolean) (ElapsedSeconds :type Float%20%28double-precision%29) (TriggeredSeconds :type Float%20%28double-precision%29) (InputAction :type Input%20Action%20Object%20Reference :default "/Game/Input/Actions/IA_Ability_AOE_FireArrows.IA_Ability_AOE_FireArrows"))
  ;[0.15 0.15 0.15 0.5] Abilities
  (:Started
    (Class|OryxAbilityComponent|TryActivateAbility (Variables|Default|GetAbilityComponent) 4)))

(event Input|EnhancedActionEvents|EnhancedInputActionIA_Ability_AOE_IceSpiral
  (params (ActionValue :type Boolean) (ElapsedSeconds :type Float%20%28double-precision%29) (TriggeredSeconds :type Float%20%28double-precision%29) (InputAction :type Input%20Action%20Object%20Reference :default "/Game/Input/Actions/IA_Ability_AOE_IceSpiral.IA_Ability_AOE_IceSpiral"))
  ;[0.15 0.15 0.15 0.5] Abilities
  (:Started
    (Class|OryxAbilityComponent|TryActivateAbility (Variables|Default|GetAbilityComponent) 5)))

(event Input|EnhancedActionEvents|EnhancedInputActionIA_Ability_AOE_PoisonCarousel
  (params (ActionValue :type Boolean) (ElapsedSeconds :type Float%20%28double-precision%29) (TriggeredSeconds :type Float%20%28double-precision%29) (InputAction :type Input%20Action%20Object%20Reference :default "/Game/Input/Actions/IA_Ability_AOE_PoisonCarousel.IA_Ability_AOE_PoisonCarousel"))
  ;[0.15 0.15 0.15 0.5] Abilities
  (:Started
    (Class|OryxAbilityComponent|TryActivateAbility (Variables|Default|GetAbilityComponent) 6)))

(event EventBeginPlay
  (Utilities|FlowControl|Sequence
    (:then_0
      (EventDispatchers|BindEventtoOnDamageReceived (Variables|Default|GetHealthComponent) (delegate Custom|HandleDamageReceived)))
    (:then_1
      (if (Pawn|IsLocallyControlled)
        (bind _asplayer_controller (Utilities|Casting|CastToPlayerController (Pawn|GetController)))
        (Input|SetInputModeGameOnly _asplayer_controller false)
        (Variables|/Script/Engine.PlayerController|SetbShowMouseCursor _asplayer_controller false)))))

(event EventOnToggleStatsScreen
  ;[0.15 0.15 0.15 0.5] Enable/Disable Stats
  (Utilities|IsValid (Variables|Default|GetStatsScreenInstance)
    (:Is%20Valid
      (Widget|RemovefromParent (Variables|Default|GetStatsScreenInstance))
      (Variables|Default|SetStatsScreenInstance 0))
    (:Is%20Not%20Valid
      (bind _returnvalue (UserInterface|CreateWidget "/Game/UI/HUD/Widgets/WBP_StatsScreen.WBP_StatsScreen_C" (.AsPlayer%20Controller (Utilities|Casting|CastToPlayerController (Pawn|GetController)))))
      (UserInterface|Viewport|AddtoViewport _returnvalue 0)
      (Variables|Default|SetStatsScreenInstance _returnvalue))))

(fn ConstructionScript)